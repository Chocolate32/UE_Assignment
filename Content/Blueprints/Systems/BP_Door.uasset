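; BP_Door is a double door with a text label that slides its two frames to an open position when interacted with.
; The Interact event moves LeftFrame and RightFrame over TimeToOpen, deriving the left target by negating the X of RightTargetPostion.
; The construction script writes the Text variable to the TextRender component; the graph has no closing logic.
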(event `/Game/Blueprints/Systems/BPI_Interact.Interact`
  (bind (_righttargetpostion_x _righttargetpostion_y _righttargetpostion_z) (`KismetMathLibrary.BreakVector` (`self.RightTargetPostion`)))
  (bind _timetoopen (`self.TimeToOpen`))
  (`|ExecutionSequence`
    (:`then_0`
      (`KismetSystemLibrary.MoveComponentTo` (`self.LeftFrame`) (`KismetMathLibrary.MakeVector` (* _righttargetpostion_x -1.0) _righttargetpostion_y _righttargetpostion_z) (struct) false false _timetoopen))
    (:`then_1`
      (`KismetSystemLibrary.MoveComponentTo` (`self.RightFrame`) (`self.RightTargetPostion`) (struct) false false _timetoopen))))

(fn `UserConstructionScript`
  (`TextRenderComponent.K2_SetText` (`self.TextRender`) (`self.Text`)))