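; Interactive panel that unlocks linked actors once a character has gathered enough of a tagged objective.
; Construction sets the idle text and reads the required count from ability data by Tag.
; Character collision compares the player's tagged count to it, showing a "require more" prompt until the character leaves, or calling Interact.
; Interact messages every InteractionActor, shows the validation text and destroys its collision component, making it one-shot.
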(event `self.ReceiveBeginPlay`)

(event `self.CustomBoxCollisionOnCharacter.OnCharacterCollided`
  (params (Player :type "UE_AssignmentCharacter Object Reference"))
  (`self.Player`
    (:`then`)
    (:`else`
      (bind _output_get (set `self.Player` Player))
      (bind _amount (message `/Game/Blueprints/Character/BPI_PlayerCharacter.GetAmountPerObjective` _output_get (`self.Tag`)))
      (bind _output_get_2 (set `self.Short` (< _amount (`self.Total Count`))))
      (if _output_get_2
        (`TextRenderComponent.K2_SetText` (`self.TextRender`) (`|FormatText` "You require More!"))
        (else
          (`/Game/Blueprints/Systems/BPI_Interact.Interact`))))))

(event `self.CustomBoxCollisionOnCharacter.OnCharacterLeftCollision`
  (params (Player :type "UE_AssignmentCharacter Object Reference"))
  (if (`self.Short`)
    (set `self.Player` null)
    (`TextRenderComponent.K2_SetText` (`self.TextRender`) (`self.Text`))))

(event `/Game/Blueprints/Systems/BPI_Interact.Interact`
  (for _array_element (`self.InteractionActors`)
    (message `/Game/Blueprints/Systems/BPI_Interact.Interact` _array_element))
  (`TextRenderComponent.K2_SetText` (`self.TextRender`) (`self.ValidationText`))
  (`ActorComponent.K2_DestroyComponent` (`self.CustomBoxCollisionOnCharacter`)))

(fn `UserConstructionScript`
  (`TextRenderComponent.K2_SetText` (`self.TextRender`) (`self.Text`))
  (set `self.Total Count` (`.TotalCount_30_0067ADE544F78ECBFDD093B1224F6338` (break `/Game/Blueprints/Misc/Struct_AbilityData` (`/Game/Blueprints/Extra/BFL_CasualFuncs.Get_AbilityData` (`self.Tag`))))))