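; BP_SafeLight is a spotlight actor that keeps a capsule at the point where its light hits the level, presumably marking a safe area.
; PutCapsuleOnTheGround traces on Visibility along the spotlight's forward vector for Strength units, then moves the capsule to the impact point plus Offset.
; It runs in the construction script and at BeginPlay, so placement updates in the editor but does not follow the light every frame.
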(event `self.ReceiveBeginPlay`
  (`self.PutCapsuleOnTheGround`))

(fn `PutCapsuleOnTheGround`
  (bind _spotlight (`self.SpotLight`))
  (bind _returnvalue (`SceneComponent.K2_GetComponentLocation` _spotlight))
  (bind _outhit (`KismetSystemLibrary.LineTraceSingle` _returnvalue (+ _returnvalue (* (`SceneComponent.GetForwardVector` _spotlight) (`self.Strength`))) "TraceTypeQuery1"))
  (`SceneComponent.K2_SetWorldLocationAndRotation` :`self` (`self.Capsule`) :`NewLocation` (+ (`.ImpactPoint` (`GameplayStatics.BreakHitResult` _outhit)) (`self.Offset`))))

(fn `UserConstructionScript`
  (`self.PutCapsuleOnTheGround`))